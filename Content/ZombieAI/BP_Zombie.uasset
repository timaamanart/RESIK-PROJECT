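; BP_Zombie is an enemy zombie character that targets the player, makes melee attacks and dies into a ragdoll.
; Its detection sphere sets the Blackboard TargetActor, while a looping timer updates CanAttack from player distance for BP_ZombieAIController.
; ZombieAttack halts movement, plays a montage and deals delayed damage if still in range, restoring walking only on a hit.
; AnyDamage reduces health, then at zero enables ragdoll physics and destroys the actor after a delay.
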(event `ZombieAttack`
  (if (not (`self.IsAttacking`))
    (set `self.IsAttacking` true)
    (`Controller.StopMovement` (`self.GetController`))
    (`CharacterMovementComponent.DisableMovement` (`self.CharacterMovement`))
    (`self.PlayAnimMontage` "/Game/ZombieAI/zomi/ZomAttack.ZomAttack")
    (`KismetSystemLibrary.Delay` 1.5)
    (if (<= (`self.GetDistanceTo` (`GameplayStatics.GetPlayerCharacter` 0)) 130.0)
      (`GameplayStatics.ApplyDamage` (`GameplayStatics.GetPlayerCharacter` 0) 25.0 (`self.GetController`) self)
      (`KismetSystemLibrary.Delay` 1.5)
      (`CharacterMovementComponent.SetMovementMode` (`self.CharacterMovement`) "MOVE_Walking" 0)
      (set `self.IsAttacking` false)
      (else
        (`KismetSystemLibrary.Delay` 1.5)
        (set `self.IsAttacking` false)))))

(event `self.ReceiveBeginPlay`
  (`KismetSystemLibrary.K2_SetTimer` null "CheckAttackDistance" 0.2 true))

(event `self.DetectionSphere.OnComponentBeginOverlap`
  (params (OverlappedComponent :type "PrimitiveComponent Object Reference") (OtherActor :type "Actor Object Reference") (OtherComp :type "PrimitiveComponent Object Reference") (OtherBodyIndex :type Integer) (bFromSweep :type Boolean) (SweepResult :type "HitResult Structure (by ref)"))
  (cast `/Game/ThirdPerson/Blueprints/BP_ThirdPersonCharacter` OtherActor)
  (cast `/Game/ZombieAI/BP_ZombieAIController` (`self.GetController`))
  (`BlackboardComponent.SetValueAsObject` (`AIBlueprintHelperLibrary.GetBlackboard` null) "TargetActor" OtherActor))

(event `self.ReceiveAnyDamage`
  (params (Damage :type "Float (single-precision)") (DamageType :type "DamageType Object Reference") (InstigatedBy :type "Controller Object Reference") (DamageCauser :type "Actor Object Reference"))
  (bind _mesh (`self.Mesh`))
  (bind _output_get (set `self.ZombieHealth` (- (`self.ZombieHealth`) Damage)))
  (if (<= _output_get 0.0)
    (set `self.IsDead` true)
    (`Controller.StopMovement` (`self.GetController`))
    (`CharacterMovementComponent.DisableMovement` (`self.CharacterMovement`))
    (`PrimitiveComponent.SetSimulatePhysics` _mesh true)
    (`PrimitiveComponent.SetCollisionProfileName` _mesh "ragdoll" true)
    (`PrimitiveComponent.SetCollisionEnabled` (`self.CapsuleComponent`) "NoCollision")
    (`KismetSystemLibrary.Delay` 3.0)
    (`self.K2_DestroyActor`)))

(fn `CheckAttackDistance`
  (bind _asbp_zombie_aicontroller (cast `/Game/ZombieAI/BP_ZombieAIController` (`self.GetController`)))
  (`BlackboardComponent.SetValueAsBool` (`AIBlueprintHelperLibrary.GetBlackboard` _asbp_zombie_aicontroller) "CanAttack" (<= (`self.GetDistanceTo` (`GameplayStatics.GetPlayerCharacter` 0)) 130.0)))

(fn `UserConstructionScript`)