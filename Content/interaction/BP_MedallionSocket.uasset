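; BP_MedallionSocket is a puzzle socket that accepts an inventory item of a required type and reveals its medallion mesh.
; A box overlap registers or clears it as the third-person character's current socket.
; PlaceMedallion validates the given item, consumes it, and at three placed medallions shows the game-won widget and pauses.
; A separate Interact event scans the inventory for a match but does not update the win count.
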(event `/Game/interaction/BPI_Interact.Interact`
  (params (PlayerRef :type "/Game/ThirdPerson/Blueprints/BP_ThirdPersonCharacter Object Reference"))
  (if (not (`self.IsActivated`))
    (for (_array_element _array_index) (`/Game/ThirdPerson/Blueprints/BP_ThirdPersonCharacter.InventoryItems` PlayerRef)
      (if (`|EnumEquality` (`.Type_9_4E7F02E0406F73B76E583FAC9B06FF82` (break `/Game/interaction/key/ST_ItemData` _array_element)) (`self.RequiredType`))
        (set `self.IsActivated` true)
        (`SceneComponent.SetVisibility` (`self.MedalionMesh`) true false)
        (`/Game/ThirdPerson/Blueprints/BP_ThirdPersonCharacter.DeleteInventoryItem` PlayerRef _array_index)))))

(event `self.Box.OnComponentBeginOverlap`
  (params (OverlappedComponent :type "PrimitiveComponent Object Reference") (OtherActor :type "Actor Object Reference") (OtherComp :type "PrimitiveComponent Object Reference") (OtherBodyIndex :type Integer) (bFromSweep :type Boolean) (SweepResult :type "HitResult Structure (by ref)"))
  (`KismetSystemLibrary.PrintString` "near")
  (bind _asbp_third_person_character (cast `/Game/ThirdPerson/Blueprints/BP_ThirdPersonCharacter` OtherActor))
  (set `/Game/ThirdPerson/Blueprints/BP_ThirdPersonCharacter.CurrentMedallionSocket` self _asbp_third_person_character))

(event `self.Box.OnComponentEndOverlap`
  (params (OverlappedComponent :type "PrimitiveComponent Object Reference") (OtherActor :type "Actor Object Reference") (OtherComp :type "PrimitiveComponent Object Reference") (OtherBodyIndex :type Integer))
  (bind _asbp_third_person_character (cast `/Game/ThirdPerson/Blueprints/BP_ThirdPersonCharacter` OtherActor))
  (set `/Game/ThirdPerson/Blueprints/BP_ThirdPersonCharacter.CurrentMedallionSocket` null _asbp_third_person_character))

(fn `Place Medallion`
  (params (PlayerRef :type "/Game/ThirdPerson/Blueprints/BP_ThirdPersonCharacter Object Reference") (ItemIndex :type Integer) (ItemType :type "/Game/interaction/E_ItemType Enum" :default "NewEnumerator0"))
  (if (`self.IsActivated`)
    _
    (elif (`|EnumEquality` ItemType (`self.RequiredType`))
      (set `self.IsActivated` true)
      (`SceneComponent.SetVisibility` (`self.MedalionMesh`) true false)
      (`SceneComponent.SetHiddenInGame` (`self.MedalionMesh`) false false)
      (`/Game/ThirdPerson/Blueprints/BP_ThirdPersonCharacter.DeleteInventoryItem` PlayerRef ItemIndex)
      (bind _output_get (set `/Game/ThirdPerson/Blueprints/BP_ThirdPersonCharacter.PlacedMedallions` (+ (`/Game/ThirdPerson/Blueprints/BP_ThirdPersonCharacter.PlacedMedallions` PlayerRef) 1) PlayerRef))
      (if (>= _output_get 3)
        (bind _returnvalue (`|CreateWidget` "/Game/Widgets/WBP_GameWon.WBP_GameWon_C"))
        (`UserWidget.AddToViewport` _returnvalue 0)
        (`GameplayStatics.SetGamePaused` true)))))

(fn `UserConstructionScript`)