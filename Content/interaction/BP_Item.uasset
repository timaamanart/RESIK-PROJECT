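; BP_Item is a world pickup that shows a billboard and registers itself as the player's current interact item while they overlap its sphere.
; On Interact, a note type opens a paused note-reading widget, another type grants the shotgun, and other items go to the inventory.
; Medallion items, detected by enum name prefix, also update the "Find 3 figures" quest counter.
; All pickups except notes then destroy themselves; the construction script applies mesh and scale.
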(event `self.Sphere.OnComponentBeginOverlap`
  (params (OverlappedComponent :type "PrimitiveComponent Object Reference") (OtherActor :type "Actor Object Reference") (OtherComp :type "PrimitiveComponent Object Reference") (OtherBodyIndex :type Integer) (bFromSweep :type Boolean) (SweepResult :type "HitResult Structure (by ref)"))
  (bind _asbp_third_person_character (cast `/Game/ThirdPerson/Blueprints/BP_ThirdPersonCharacter` OtherActor))
  (set `/Game/ThirdPerson/Blueprints/BP_ThirdPersonCharacter.CurrentInteractItem` self _asbp_third_person_character)
  (set `self.PlayerRef` _asbp_third_person_character)
  (set `self.CanInteract` true)
  (`SceneComponent.SetVisibility` (`self.Billboard`) true false))

(event `self.Sphere.OnComponentEndOverlap`
  (params (OverlappedComponent :type "PrimitiveComponent Object Reference") (OtherActor :type "Actor Object Reference") (OtherComp :type "PrimitiveComponent Object Reference") (OtherBodyIndex :type Integer))
  (bind _asbp_third_person_character (cast `/Game/ThirdPerson/Blueprints/BP_ThirdPersonCharacter` OtherActor))
  (set `self.PlayerRef` null)
  (set `/Game/ThirdPerson/Blueprints/BP_ThirdPersonCharacter.CurrentInteractItem` null _asbp_third_person_character)
  (set `self.CanInteract` false)
  (`SceneComponent.SetVisibility` (`self.Billboard`) false false))

(event `/Game/interaction/BPI_Interact.Interact`
  (params (PlayerRef :type "/Game/ThirdPerson/Blueprints/BP_ThirdPersonCharacter Object Reference"))
  (bind _returnvalue (`GameplayStatics.GetPlayerController` 0))
  (bind (_name _type _icon _description _quantity _canstack _notepages) (break `/Game/interaction/key/ST_ItemData` (`self.ItemData`)))
  (`/Engine/EditorBlueprintResources/StandardMacros.IsValid` PlayerRef
    (:`Is Valid`
      (if (`|EnumEquality` _type "NewEnumerator7")
        (bind _returnvalue_2 (`|CreateWidget` "/Game/Widgets/WBP_Note.WBP_Note_C" _returnvalue))
        (`/Game/Widgets/WBP_Note.InitNote` _returnvalue_2 _notepages)
        (`UserWidget.AddToViewport` _returnvalue_2 0)
        (`WidgetBlueprintLibrary.SetInputMode_UIOnlyEx` _returnvalue null)
        (set `PlayerController.bShowMouseCursor` true _returnvalue)
        (`GameplayStatics.SetGamePaused` true)
        (else
          (if (`|EnumEquality` _type "NewEnumerator8")
            (set `/Game/ThirdPerson/Blueprints/BP_ThirdPersonCharacter.HasShotGun` true PlayerRef)
            (else
              (`/Game/ThirdPerson/Blueprints/BP_ThirdPersonCharacter.AddItemToInventory` PlayerRef (`self.ItemData`))
              (if (`KismetStringLibrary.StartsWith` (`|GetEnumeratorNameAsString` _type) "Medallion")
                (bind _asbp_third_person_character (cast `/Game/ThirdPerson/Blueprints/BP_ThirdPersonCharacter` PlayerRef))
                (bind _output_get (set `/Game/ThirdPerson/Blueprints/BP_ThirdPersonCharacter.MedallionCount` (+ (`/Game/ThirdPerson/Blueprints/BP_ThirdPersonCharacter.MedallionCount` _asbp_third_person_character) 1) _asbp_third_person_character))
                (`TextBlock.SetText` (`/Game/Widgets/WBP_Quest.QuestText` (`/Game/ThirdPerson/Blueprints/BP_ThirdPersonCharacter.QuestWidgetRef` _asbp_third_person_character)) (`|FormatText` "Find 3 figures: {Count}/3" _output_get)))))
          (`self.K2_DestroyActor`))))))

(fn `Interact Old`)

(fn `UserConstructionScript`
  (`StaticMeshComponent.SetStaticMesh` (`self.StaticMesh`) (`self.ItemMesh`))
  (`SceneComponent.SetRelativeScale3D` (`self.StaticMesh`) (`self.ItemMeshScale`)))