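; BP_Door3 is an interactable hinged door that can optionally require one of two player-held keys, selected by KeyID.
; Its Box overlap registers or clears the door as the third-person character's CurrentInteractItem.
; Interact checks the key, then toggles a timeline forward or in reverse to lerp the pivot between closed and 90-degree open rotations.
; UnlockAndOpen only clears a Locked flag, which Interact never reads.
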(event `self.ReceiveBeginPlay`
  (set `self.ClosedRot` (`SceneComponent.RelativeRotation` (`self.DoorPIvot`)))
  (set `self.OpenRot` (`KismetMathLibrary.ComposeRotators` (`self.ClosedRot`) (struct :`Yaw` 90.0))))

(event `self.Interact`
  (params (PlayerRef :type "/Game/ThirdPerson/Blueprints/BP_ThirdPersonCharacter Object Reference"))
  (if (`self.NeedKey`)
    (switch `int` (`self.KeyID`)
      (:`0`
        (if (`/Game/ThirdPerson/Blueprints/BP_ThirdPersonCharacter.HasKey1` PlayerRef)
          (if (`self.IsOpen`) :!label _label
            (set `self.IsOpen` false)
            (bind (_direction _newtrack_0) (`Timeline|TL_Door` :!via `Reverse` :!label _label_2)
              (:`Update`
                (`SceneComponent.K2_SetRelativeRotation` (`self.DoorPIvot`) (`KismetMathLibrary.RLerp` (`self.ClosedRot`) (`self.OpenRot`) _newtrack_0) false false)))
            (else
              (set `self.IsOpen` true)
              (goto _label_2)))))
      (:`1`
        (if (`/Game/ThirdPerson/Blueprints/BP_ThirdPersonCharacter.HasKey2` PlayerRef)
          (goto _label))))
    (else
      (goto _label))))

(event `self.Box.OnComponentBeginOverlap`
  (params (OverlappedComponent :type "PrimitiveComponent Object Reference") (OtherActor :type "Actor Object Reference") (OtherComp :type "PrimitiveComponent Object Reference") (OtherBodyIndex :type Integer) (bFromSweep :type Boolean) (SweepResult :type "HitResult Structure (by ref)"))
  (bind _asbp_third_person_character (cast `/Game/ThirdPerson/Blueprints/BP_ThirdPersonCharacter` OtherActor))
  (set `/Game/ThirdPerson/Blueprints/BP_ThirdPersonCharacter.CurrentInteractItem` self _asbp_third_person_character))

(event `UnlockAndOpen`
  (set `self.Locked` false))

(event `self.Box.OnComponentEndOverlap`
  (params (OverlappedComponent :type "PrimitiveComponent Object Reference") (OtherActor :type "Actor Object Reference") (OtherComp :type "PrimitiveComponent Object Reference") (OtherBodyIndex :type Integer))
  (bind _asbp_third_person_character (cast `/Game/ThirdPerson/Blueprints/BP_ThirdPersonCharacter` OtherActor))
  (set `/Game/ThirdPerson/Blueprints/BP_ThirdPersonCharacter.CurrentInteractItem` null _asbp_third_person_character))

(fn `UserConstructionScript`)